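; BP_LightDefault is a base light Blueprint in the weather/time module that spawns a configurable light component at runtime.
; On BeginPlay it adds a component of class LightType at the configured relative transform, stores it as LightComponent, then calls SetLightParams.
; SetLightParams hides the light and applies intensity, units, linear color and attenuation radius.
; Child Blueprints can add parameters and override that function.
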(event EventBeginPlay
  (bind _returnvalue (Game|AddComponentbyClass (Variables|LightSettings|GetLightType) false (Math|Transform|MakeTransform (Variables|LightSettings|GetRelative%20Transform%20Location) (Variables|LightSettings|GetRelative%20Transform%20Rotation) "1.000000,1.000000,1.000000")))
  (bind _output_get (Variables|Default|SetLightComponent _returnvalue))
  (Utilities|IsValid _output_get
    (:Is%20Valid
      (CallFunction|SetLightParams))))

(fn ConstructionScript)

(fn SetLightParams
  ;[1 1 1] Выставляем свет по параметрам, если необходимо в дочерних бп добавляем параметры и оверрайдим
  (Rendering|SetVisibility (Variables|Default|GetLightComponent) false true)
  (Class|LocalLightComponent|SetIntensityUnits (Variables|Default|GetLightComponent) (Variables|LightSettings|Get%20Intensity%20Units))
  (Rendering|Components|Light|SetIntensity (Variables|Default|GetLightComponent) (Variables|LightSettings|GetIntensity))
  (Rendering|Components|Light|SetLightColor (Variables|Default|GetLightComponent) (Variables|LightSettings|GetColor) false)
  (Rendering|Lighting|SetAttenuationRadius (Variables|Default|GetLightComponent) (Variables|LightSettings|GetAttenuationRadius)))