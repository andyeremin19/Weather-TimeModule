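; Manager actor that drives time of day and season from the weather-control widget held by the game mode, via interface messages to the level's UDS and UDW actors.
; Slider changes map to a morning-to-night time, then lerp cloud, skylight, sun, shadow and fog settings between four keyframes, adding UDW's cloudiness to cloud coverage.
; Near a threshold time it toggles local lights on light-source actors and the MPC_Weather Night parameter.
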(event Custom|OnTimeChange_Event
  (params (SliderValue :type Float%20%28double-precision%29))
  (CallFunction|ChangeTimeOfDay SliderValue))

(event Custom|OnSummer_Event
  (params (Season :type E_Seasons%20Enum :default "NewEnumerator0"))
  (Class|BPIUDW|SeasonChange(Message) (Variables|Elements|GetUDW) Season))

(event EventBeginPlay
  ;[1 1 1] Нужна будет ссылка на HUD
  (bind _asbp_third_person_game_mode (Utilities|Casting|CastToBP_ThirdPersonGameMode (Game|GetGameMode)))
  ;[1 1 1] Получаем ссылки на UD
  (CallFunction|SetWeatherReferences)
  (EventDispatchers|AssignOnTimeChange (Variables|/Game/Weather_Time_Module/Blueprints/BP_ThirdPersonGameMode.BP_ThirdPersonGameMode_C|GetBPW_WeatherControl _asbp_third_person_game_mode) (delegate Custom|OnTimeChange_Event))
  (EventDispatchers|AssignOnSeasonChange (Variables|/Game/Weather_Time_Module/Blueprints/BP_ThirdPersonGameMode.BP_ThirdPersonGameMode_C|GetBPW_WeatherControl _asbp_third_person_game_mode) (delegate Custom|OnSummer_Event)))

(fn ConstructionScript)

(fn ToggleLightsVisibility
  (params (IsVisible :type Boolean))
  (bind _lightsource (Variables|Elements|GetLightSource))
  ;[1 1 1] Включаем/Выключаем фонари, прожекторы и тд
  (Utilities|LoadClassAssetBlocking _lightsource)
  (bind _outactors (Actor|GetAllActorsOfClass (Utilities|ResolveSoftReference _lightsource)))
  (for _array_element _outactors
    (Utilities|IsValid (Actor|GetComponentbyClass _array_element "/Script/Engine.LocalLightComponent")
      (:Is%20Valid
        (Rendering|SetVisibility (Actor|GetComponentbyClass _array_element "/Script/Engine.LocalLightComponent") IsVisible true))))
  ;[1 1 1] Может вообще не понадобиться, уточнять с лвлом
  (if IsVisible
    (Rendering|Material|SetScalarParameterValue "/Game/Weather_Time_Module/Materials/MPC_Weather.MPC_Weather" "Night" 1.0 :!class /Script/Engine.KismetMaterialLibrary)
    (else
      (Rendering|Material|SetScalarParameterValue "/Game/Weather_Time_Module/Materials/MPC_Weather.MPC_Weather" "Night" 0.0 :!class /Script/Engine.KismetMaterialLibrary)))
  (Variables|Default|SetbLightsAreOn IsVisible))

(fn ChangeTimeOfDay
  (params (SliderValue :type Float%20%28double-precision%29))
  ;[1 1 1] Логика смены времени
  (Class|BPIUDS|SetTimeOfDay(Message) (Variables|Elements|GetUDS) (Math|Float|MapRangeClamped SliderValue 0.0 1.0 (Variables|TimeSettings|GetTime_M) (Variables|TimeSettings|GetTime_N)))
  (Utilities|FlowControl|Sequence
    (:then_0
      (bind _currenttime (Class|BPIUDS|GetTimeOfDay(Message) (Variables|Elements|GetUDS)))
      (if (Math|Float|NearlyEqual(Float) _currenttime (Variables|TimeSettings|GetTime_ToToggleLights) 1e+01)
        (if (Variables|Default|GetbLightsAreOn)
          (CallFunction|ToggleLightsVisibility false)
          (else
            (CallFunction|ToggleLightsVisibility true)))))
    (:then_1
      (bind (_cloudcoverage _skylightintensity _cloudshadowsintensity _sunlightintensity _fogdensity) (CallFunction|CalculateWeatherChange))
      (Class|BPIUDS|SetUDSValues(Message) (Variables|Elements|GetUDS) _cloudcoverage _skylightintensity _cloudshadowsintensity _sunlightintensity _fogdensity))))

(fn SetWeatherReferences
  (bind _udwsc (Variables|Elements|GetUDWsc))
  (bind _udssc (Variables|Elements|GetUDSsc))
  (Utilities|LoadClassAssetBlocking _udssc)
  (bind _returnvalue (Actor|GetActorOfClass (Utilities|ResolveSoftReference _udssc)))
  (Variables|Elements|SetUDS _returnvalue)
  (Utilities|LoadClassAssetBlocking _udwsc)
  (bind _returnvalue_2 (Actor|GetActorOfClass (Utilities|ResolveSoftReference _udwsc)))
  (Variables|Elements|SetUDW _returnvalue_2))

(fn CalculateWeatherChange
  (bind _currenttime (Class|BPIUDS|GetTimeOfDay(Message) (Variables|Elements|GetUDS)))
  (LocalVariables|SetTimeOfDay _currenttime)
  (if (>= (LocalVariables|GetTimeOfDay) (Variables|TimeSettings|GetTime_E))
    ;[1 1 1] Вечер-Ночь
    (LocalVariables|SetCloudCov (Math|Float|MapRangeClamped (LocalVariables|GetTimeOfDay) (Variables|TimeSettings|GetTime_E) (Variables|TimeSettings|GetTime_N) (Variables|TimeSettings|GetCloudCoverage_E) (Variables|TimeSettings|GetCloudCoverage_N)))
    (LocalVariables|SetSkylightInt (Math|Float|MapRangeClamped (LocalVariables|GetTimeOfDay) (Variables|TimeSettings|GetTime_E) (Variables|TimeSettings|GetTime_N) (Variables|TimeSettings|GetSkyLightIntensity_E) (Variables|TimeSettings|GetSkyLightIntensity_N)))
    (LocalVariables|SetCloudShadows (Math|Float|MapRangeClamped (LocalVariables|GetTimeOfDay) (Variables|TimeSettings|GetTime_E) (Variables|TimeSettings|GetTime_N) (Variables|TimeSettings|GetCloudShadows_E) (Variables|TimeSettings|GetCloudShadows_N)))
    (LocalVariables|SetSunlightInt (Math|Float|MapRangeClamped (LocalVariables|GetTimeOfDay) (Variables|TimeSettings|GetTime_E) (Variables|TimeSettings|GetTime_N) (Variables|TimeSettings|GetSunlightInt_E) (Variables|TimeSettings|GetSunlightInt_N)))
    (LocalVariables|SetFogDens (Math|Float|MapRangeClamped (LocalVariables|GetTimeOfDay) (Variables|TimeSettings|GetTime_E) (Variables|TimeSettings|GetTime_N) (Variables|TimeSettings|GetFogDensity_E) (Variables|TimeSettings|GetFogDensity_N)))
    (elif (>= (LocalVariables|GetTimeOfDay) (Variables|TimeSettings|GetTime_D))
      ;[1 1 1] День-Вечер
      (LocalVariables|SetCloudCov (Math|Float|MapRangeClamped (LocalVariables|GetTimeOfDay) (Variables|TimeSettings|GetTime_D) (Variables|TimeSettings|GetTime_E) (Variables|TimeSettings|GetCloudCoverage_D) (Variables|TimeSettings|GetCloudCoverage_E)))
      (LocalVariables|SetSkylightInt (Math|Float|MapRangeClamped (LocalVariables|GetTimeOfDay) (Variables|TimeSettings|GetTime_D) (Variables|TimeSettings|GetTime_E) (Variables|TimeSettings|GetSkyLightIntensity_D) (Variables|TimeSettings|GetSkyLightIntensity_E)))
      (LocalVariables|SetCloudShadows (Math|Float|MapRangeClamped (LocalVariables|GetTimeOfDay) (Variables|TimeSettings|GetTime_D) (Variables|TimeSettings|GetTime_E) (Variables|TimeSettings|GetCloudShadows_D) (Variables|TimeSettings|GetCloudShadows_E)))
      (LocalVariables|SetSunlightInt (Math|Float|MapRangeClamped (LocalVariables|GetTimeOfDay) (Variables|TimeSettings|GetTime_D) (Variables|TimeSettings|GetTime_E) (Variables|TimeSettings|GetSunlightInt_D) (Variables|TimeSettings|GetSunlightInt_E)))
      (LocalVariables|SetFogDens (Math|Float|MapRangeClamped (LocalVariables|GetTimeOfDay) (Variables|TimeSettings|GetTime_D) (Variables|TimeSettings|GetTime_E) (Variables|TimeSettings|GetFogDensity_D) (Variables|TimeSettings|GetFogDensity_E)))
      (else
        ;[1 1 1] Утро-День
        (LocalVariables|SetCloudCov (Math|Float|MapRangeClamped (LocalVariables|GetTimeOfDay) (Variables|TimeSettings|GetTime_M) (Variables|TimeSettings|GetTime_D) (Variables|TimeSettings|GetCloudCoverage_M) (Variables|TimeSettings|GetCloudCoverage_D)))
        (LocalVariables|SetSkylightInt (Math|Float|MapRangeClamped (LocalVariables|GetTimeOfDay) (Variables|TimeSettings|GetTime_M) (Variables|TimeSettings|GetTime_D) (Variables|TimeSettings|GetSkyLightIntensity_M) (Variables|TimeSettings|GetSkyLightIntensity_D)))
        (LocalVariables|SetCloudShadows (Math|Float|MapRangeClamped (LocalVariables|GetTimeOfDay) (Variables|TimeSettings|GetTime_M) (Variables|TimeSettings|GetTime_D) (Variables|TimeSettings|GetCloudShadows_M) (Variables|TimeSettings|GetCloudShadows_D)))
        (LocalVariables|SetSunlightInt (Math|Float|MapRangeClamped (LocalVariables|GetTimeOfDay) (Variables|TimeSettings|GetTime_M) (Variables|TimeSettings|GetTime_D) (Variables|TimeSettings|GetSunlightInt_M) (Variables|TimeSettings|GetSunlightInt_D)))
        (LocalVariables|SetFogDens (Math|Float|MapRangeClamped (LocalVariables|GetTimeOfDay) (Variables|TimeSettings|GetTime_M) (Variables|TimeSettings|GetTime_D) (Variables|TimeSettings|GetFogDensity_M) (Variables|TimeSettings|GetFogDensity_D))))))
  (bind _cloudnesscoef (Class|BPIUDW|GetCurrentCloudnessCoef(Message) (Variables|Elements|GetUDW)))
  (return (+ _cloudnesscoef (LocalVariables|GetCloudCov)) (LocalVariables|GetSkylightInt) (LocalVariables|GetCloudShadows) (LocalVariables|GetSunlightInt) (LocalVariables|GetFogDens)))

(fn GetInitialTime
  ;[1 1 1] Устанавливает слайдер в значение равное начальному времени на карте
  (bind _currenttime (Class|BPIUDS|GetTimeOfDay(Message) (Variables|Elements|GetUDS)))
  (return (Math|Float|MapRangeClamped _currenttime (Variables|TimeSettings|GetTime_M) (Variables|TimeSettings|GetTime_N) 0.0 1.0)))